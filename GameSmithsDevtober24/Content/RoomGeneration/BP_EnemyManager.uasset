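; BP_EnemyManager spawns enemies at supplied location points for room generation.
; On BeginPlay it builds a class-to-weight map from the SpawnRatesDT data table.
; SpawnallEnemies picks each enemy class by cumulative weighted random, places it at a random point and removes a random point from the list, capping the count at available points.
; SpawnEnemiesAtPoints works similarly but always spawns BP_Enemy_Normal_Child.
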(event Custom|Spawn%20all%20Enemies
  (params (Spawn%20Locations :type Array%20of%20Scene%20Component%20Object%20References) (NumEnemies :type Integer))
  (bind (_outitem _outindex) (Utilities|Array|Random Spawn%20Locations))
  (for _index (range 0 (Math|Integer|Min(Integer) NumEnemies (Utilities|Array|Length Spawn%20Locations)))
    (bind _selected_class (CallFunction|WeightedRandom (Variables|Default|GetEnemySpawnRateMap)))
    (Game|SpawnActorfromClass _selected_class (Transformation|GetWorldTransform _outitem) "Undefined" "MultiplyWithRoot" 0 0)
    (Utilities|Array|RemoveIndex Spawn%20Locations _outindex)))

(event EventBeginPlay
  (bind _spawn_rates_dt (Variables|Default|GetSpawn%20Rates%20DT))
  (bind _outrownames (DataTable|GetDataTableRowNames _spawn_rates_dt))
  (for _array_element _outrownames
    (bind _returnvalue (Utilities|GetDataTableRow _spawn_rates_dt _array_element)
      (:then
        (Utilities|Map|Add (Variables|Default|GetEnemySpawnRateMap) (.RoomClass (Utilities|Struct|BreakE_EnemyWeightEntry _returnvalue)) (.Weight (Utilities|Struct|BreakE_EnemyWeightEntry _returnvalue)))))))

(fn ConstructionScript)

(fn SpawnEnemiesatPoints
  (params (Positions :type Array%20of%20Scene%20Component%20Object%20References) (TotalEnemyCount :type Integer))
  (bind _output_get (LocalVariables|SetRemainingPositions Positions))
  (for _index (range 0 TotalEnemyCount)
    (if (> (Utilities|Array|Length _output_get) 0)
      (bind _output_get_2 (LocalVariables|SetCurrentTransform (Transformation|GetWorldTransform (.OutItem (Utilities|Array|Random _output_get)))))
      (Utilities|Array|RemoveIndex _output_get (.OutIndex (Utilities|Array|Random _output_get)))
      (Game|SpawnActorfromClass "/Game/Mechanics/Enemies/BP_Enemy_Normal_Child.BP_Enemy_Normal_Child_C" _output_get_2 "Undefined" "MultiplyWithRoot" 0 0))))

(fn WeightedRandom
  (params (Selection :type Map%20of%20BP%20Enemy%20Template%20Class%20References%20to%20Reals))
  ;[0.3025 0.4105 0.7083] Random selection from weights (higher is more common)
  (bind _keys (Utilities|Map|Keys Selection))
  (for _array_element _keys
    (bind _output_get (Variables|Default|SetCounter (+ (stale _output_get) (.Value (Utilities|Map|Find Selection _array_element))))))
  (Variables|Default|SetChosen (Math|Random|RandomFloatinRange 0.0 (Variables|Default|GetCounter)))
  (bind _keys_2 (Utilities|Map|Keys Selection))
  (for _array_element_2 _keys_2
    (bind _output_get_2 (Variables|Default|SetCounter (- (Variables|Default|GetCounter) (.Value (Utilities|Map|Find Selection _array_element_2)))))
    (if (<= _output_get_2 (Variables|Default|GetChosen))
      (return _array_element_2))))