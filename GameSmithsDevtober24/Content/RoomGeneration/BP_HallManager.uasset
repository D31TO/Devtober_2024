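; BP_HallManager procedurally builds a level hall as a chain of rooms, weighted by the RoomSet table.
; Each room spawns at the previous out connector, and is rejected if it overlaps or exceeds the remaining player shell budget.
; Repeated failures backtrack one room, restoring its saved exclusions and attempt count.
; At target length it teleports the player to the start, places the level end, lights rooms and triggers enemy and shell spawning.
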(event Custom|On%20Next%20Room%20Req
  (params (Random%20Seed :type Random%20Stream%20Structure) (Previous%20Room :type BP%20Hall%20Template%20Object%20Reference) (Spawn%20At%20Component :type Scene%20Component%20Object%20Reference))
  (bind _spawnedrooms (Variables|Default|GetSpawnedRooms))
  ;[1 0.2302 0.4592] Room Generation
  (Utilities|IsValid Previous%20Room
    (:Is%20Valid
      (bind _output_get (Variables|Default|SetSpawnTransform (Transformation|GetWorldTransform Spawn%20At%20Component))))
    (:Is%20Not%20Valid
      (Variables|Default|SetSpawnTransform (Variables|Default|GetStartTransform))))
  (bind _selected_room (CallFunction|WeightedRoomRandomisation (Variables|Default|GetMapSet) Random%20Seed (Variables|Default|GetGlobalDisallowedRooms)))
  (bind _returnvalue (Game|SpawnActorfromClass _selected_room _output_get "Undefined" "MultiplyWithRoot" 0 Previous%20Room 0))
  (Utilities|IsValid Previous%20Room
    (:Is%20Valid
      (Default|RemoveComponents _returnvalue false))
    (:Is%20Not%20Valid
      (Variables|Default|SetFirstRoom _returnvalue)))
  (bind _any_overlaps (Default|GetOverlappingActors _returnvalue))
  (if _any_overlaps
    (Utilities|Set|Add (Variables|Default|GetGlobalDisallowedRooms) _selected_room :!label _label)
    (Actor|DestroyActor _returnvalue)
    (bind _result (Math|Integer|IncrementInt (Variables|Default|GetFailedAttempts))
      (:%20%20
        (if (> _result (Variables|Default|GetBacktrackAfterNumAttempts))
          (bind _output_get_2 (Variables|Default|SetRoomBuffer (Variables|/Game/RoomGeneration/BP_HallTemplate.BP_HallTemplate_C|GetPrevious%20Room Previous%20Room)))
          (Actor|DestroyActor Previous%20Room)
          (Variables|Default|SetFailedAttempts (Variables|/Game/RoomGeneration/BP_HallTemplate.BP_HallTemplate_C|GetAttemptsBeforeSpawn _output_get_2))
          (Variables|Default|SetMaxNumberShells (+ (Variables|Default|GetMaxNumberShells) (Variables|/Game/RoomGeneration/BP_HallTemplate.BP_HallTemplate_C|GetShellsToComplete _output_get_2)))
          (Variables|Default|SetGlobalDisallowedRooms (Variables|/Game/RoomGeneration/BP_HallTemplate.BP_HallTemplate_C|GetDisallowedRooms _output_get_2))
          (Default|CallOnNextRoomRequest Random%20Seed _output_get_2 (Default|GetOUTConnector _output_get_2))
          (else
            (Default|CallOnNextRoomRequest Random%20Seed Previous%20Room Spawn%20At%20Component)))))
    (elif (<= (Variables|/Game/RoomGeneration/BP_HallTemplate.BP_HallTemplate_C|GetShellsToComplete _returnvalue) (Variables|Default|GetMaxNumberShells))
      (Variables|Default|SetMaxNumberShells (- (Variables|Default|GetMaxNumberShells) (Variables|/Game/RoomGeneration/BP_HallTemplate.BP_HallTemplate_C|GetShellsToComplete _returnvalue)))
      (Utilities|Array|Add _spawnedrooms _returnvalue)
      (if (< (Utilities|Array|Length _spawnedrooms) (Variables|Default|GetMaxSequenceLength))
        (Variables|/Game/RoomGeneration/BP_HallTemplate.BP_HallTemplate_C|SetDisallowedRooms _returnvalue (Variables|Default|GetGlobalDisallowedRooms))
        (Variables|/Game/RoomGeneration/BP_HallTemplate.BP_HallTemplate_C|SetAttemptsBeforeSpawn _returnvalue (Variables|Default|GetFailedAttempts))
        (Variables|Default|SetGlobalDisallowedRooms (Utilities|Set|MakeSet))
        (Variables|Default|SetFailedAttempts 0)
        (Utilities|FlowControl|DelayUntilNextTick)
        (Variables|Default|SetRoomBuffer 0)
        (Default|RemoveComponents _returnvalue true)
        (Default|CallOnNextRoomRequest Random%20Seed _returnvalue (Default|GetOUTConnector _returnvalue))
        (else
          (Development|PrintString "Completed")
          (Default|CallOnGenerationCompleted (Variables|Default|GetFirstRoom) _returnvalue)))
      (else
        (goto _label)))))

(event Custom|On%20Hall%20Generation%20Completed
  (params (Start%20Room :type BP%20Hall%20Template%20Object%20Reference) (End%20Room :type BP%20Hall%20Template%20Object%20Reference))
  (bind _allenemyspawnlocations (Variables|Default|GetAllEnemySpawnLocations))
  (bind _allshellspawnlocations (Variables|Default|GetAllShellSpawnLocations))
  (bind _returnvalue (Actor|GetActorOfClass "/Game/FirstPerson/Blueprints/BP_FirstPersonCharacter.BP_FirstPersonCharacter_C"))
  (Utilities|IsValid _returnvalue
    (:Is%20Valid
      (Transformation|SetActorTransform _returnvalue (Transformation|GetWorldTransform (Variables|/Game/RoomGeneration/BP_HallTemplate.BP_HallTemplate_C|GetPlayerSpawnLocation Start%20Room)) false true))
    (:Is%20Not%20Valid
      _))
  (Game|SpawnActorfromClass "/Game/TouchPads/EndLevel.EndLevel_C" (Transformation|GetWorldTransform (Variables|/Game/RoomGeneration/BP_HallTemplate.BP_HallTemplate_C|GetFinishSpawnLocation End%20Room)) "Undefined" "MultiplyWithRoot" 0 0)
  (bind _returnvalue_2 (Actor|GetActorOfClass "/Game/RoomGeneration/BP_EnemyManager.BP_EnemyManager_C"))
  (Utilities|IsValid _returnvalue_2
    (:Is%20Valid
      (for _array_element (Variables|Default|GetSpawnedRooms)
        (Utilities|IsValid _array_element
          (:Is%20Valid
            (Utilities|Array|AppendArray _allenemyspawnlocations (Components|GetChildrenComponents (Variables|/Game/RoomGeneration/BP_HallTemplate.BP_HallTemplate_C|GetEnemySpawnLocations _array_element) true))
            (Default|LetTherebeLight _array_element)
            (Utilities|Array|AppendArray _allshellspawnlocations (Components|GetChildrenComponents (Variables|/Game/RoomGeneration/BP_HallTemplate.BP_HallTemplate_C|GetShellSpawns _array_element) true)))))
      (Default|SpawnAllEnemies _returnvalue_2 _allenemyspawnlocations (Math|Random|RandomIntegerinRange 2 (Math|Float|Round (/ (Utilities|Array|Length _allenemyspawnlocations) 3))))
      (bind _returnvalue_3 (Actor|GetActorOfClass "/Game/RoomGeneration/BP_ShellManager.BP_ShellManager_C"))
      (Default|SpawnShells _returnvalue_3 _allshellspawnlocations (Math|Random|RandomIntegerinRange 3 (Math|Float|Round (/ (Utilities|Array|Length _allshellspawnlocations) 3)))))))

(event EventBeginPlay
  (bind _roomset (Variables|Default|GetRoomSet))
  ;[0.4854 1 0.3984] Startup
  (Variables|Default|SetRandom%20Seed (Math|Random|MakeRandomStream (Math|Random|RandomIntegerinRange -10000 10000)))
  (Utilities|FlowControl|DelayUntilNextTick)
  (Utilities|FlowControl|Sequence
    (:then_0
      (EventDispatchers|BindEventtoOnNextRoomRequest (EventDispatchers|CreateEvent :!event Custom|On%20Next%20Room%20Req))
      (EventDispatchers|BindEventtoOnGenerationCompleted (EventDispatchers|CreateEvent :!event Custom|On%20Hall%20Generation%20Completed)))
    (:then_1
      (bind _outrownames (DataTable|GetDataTableRowNames _roomset))
      (for _array_element _outrownames
        (bind _returnvalue (Utilities|GetDataTableRow _roomset _array_element)
          (:then
            (Utilities|Map|Add (Variables|Default|GetMapSet) (.RoomClass (Utilities|Struct|BreakE_HallWeightEntry _returnvalue)) (.Weight (Utilities|Struct|BreakE_HallWeightEntry _returnvalue))))))
      (bind _returnvalue_2 (Actor|GetActorOfClass "/Game/FirstPerson/Blueprints/BP_FirstPersonCharacter.BP_FirstPersonCharacter_C"))
      (Utilities|IsValid _returnvalue_2
        (:Is%20Valid
          (Variables|Default|SetMaxNumberShells (Variables|/Game/FirstPerson/Blueprints/BP_Weapon_Component.BP_Weapon_Component_C|GetShells (Variables|/Game/FirstPerson/Blueprints/BP_FirstPersonCharacter.BP_FirstPersonCharacter_C|GetWeaponComponent _returnvalue_2)))
          (Default|CallOnNextRoomRequest (Variables|Default|GetRandom%20Seed)))))))

(fn ConstructionScript)

(fn WeightedRoomRandomisation
  (params (Room%20Selection :type Map%20of%20BP%20Hall%20Template%20Class%20References%20to%20Reals) (Random%20Stream :type Random%20Stream%20Structure) (DisallowedRooms :type Set%20of%20BP%20Hall%20Template%20Class%20References))
  ;[0.3025 0.4105 0.7083] Random selection from weights (higher is more common)
  (bind _keys (Utilities|Map|Keys Room%20Selection))
  (for _array_element _keys
    (if (Utilities|Set|Contains DisallowedRooms _array_element)
      (Development|PrintString "room disallowed, skipping")
      (else
        (bind _output_get (LocalVariables|SetCounter (+ (stale _output_get) (.Value (Utilities|Map|Find Room%20Selection _array_element))))))))
  (LocalVariables|SetChosen (Math|Random|RandomFloatinRange 0.0 (LocalVariables|GetCounter)))
  (bind _keys_2 (Utilities|Map|Keys Room%20Selection))
  (for _array_element_2 _keys_2
    (bind _output_get_2 (LocalVariables|SetCounter (- (LocalVariables|GetCounter) (.Value (Utilities|Map|Find Room%20Selection _array_element_2)))))
    (if (<= _output_get_2 (LocalVariables|GetChosen))
      (return _array_element_2))))

(fn AttemptSpawnatConnector
  (params (Room%20to%20Spawn :type BP%20Hall%20Template%20Object%20Reference) (Previous%20Room%20Connector :type Scene%20Component%20Object%20Reference)))

(fn TFlip
  (params (In :type Transform))
  (bind (_location _rotation) (Math|Transform|BreakTransform In))
  (return (Math|Transform|MakeTransform _location (Math|Rotator|CombineRotators _rotation "0.000000,180.000000,0.000000"))))

(fn WeightedRoomRandomisation2
  (params (Room%20Selection :type Map%20of%20BP%20Hall%20Template%20Class%20References%20to%20Reals) (Random%20Stream :type Random%20Stream%20Structure) (DisallowedRooms :type Set%20of%20BP%20Hall%20Template%20Class%20References))
  ;[0.3025 0.4105 0.7083] Random selection from weights (higher is more common)
  (bind _keys (Utilities|Map|Keys Room%20Selection))
  (for _array_element _keys
    (if (Utilities|Set|Contains DisallowedRooms _array_element)
      (Development|PrintString "contains")
      (else
        (for _index (range 0 (Math|Float|Round (.Value (Utilities|Map|Find Room%20Selection _array_element))))
          (Utilities|Array|Add (LocalVariables|GetSelection) _array_element)
          (Development|PrintString (Utilities|GetClassDisplayName _array_element))))))
  (return (.OutItem (Utilities|Array|Random (LocalVariables|GetSelection)))))