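; BP_HallTemplate is a hall piece for room generation that snaps onto connector components and reports whether it fits.
; PositionToComponent re-origins the root by inverting a connector's relative transform, moves to the target, and retries rotated 180 degrees if Hitbox overlaps.
; Helpers report halls overlapping PositionalValidators, expose the out connector and remove in or out components.
; LetThereBeLight spawns rect lights at LightPoint children; SetTransform is used only by unreachable code.
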(event Custom|Let%20There%20Be%20Light
  (for _array_element (Components|GetChildrenComponents (Variables|Default|GetLightPoint) true)
    (bind _returnvalue (Game|SpawnActorfromClass "/Script/Engine.RectLight" (Transformation|GetWorldTransform _array_element) "Undefined" "MultiplyWithRoot" 0 0))
    (Rendering|Components|Light|SetIntensity (Variables|/Script/Engine.RectLight|GetRectLightComponent _returnvalue) 5e+03)))

(event EventBeginPlay
  (CallFunction|SetorResetOrigin (Variables|Default|GetInConnector) false))

(fn ConstructionScript)

(fn PositiontoComponent
  (params (Component%20to%20Spawn%20At :type Scene%20Component%20Object%20Reference) (Component%20to%20use%20as%20Origin :type Scene%20Component%20Object%20Reference))
  (bind _returnvalue (Transformation|GetActorTransform))
  (bind (_location _rotation) (Math|Transform|BreakTransform _returnvalue))
  (CallFunction|SetorResetOrigin Component%20to%20use%20as%20Origin false)
  (Transformation|SetActorTransform (Transformation|GetWorldTransform Component%20to%20Spawn%20At))
  (if (== (Utilities|Array|Length (Collision|GetOverlappingActors (Variables|Default|GetHitbox) 0 :!class /Script/Engine.PrimitiveComponent)) 0)
    _
    (else
      (Transformation|SetActorTransform (Math|Transform|MakeTransform _location (Math|Rotator|CombineRotators _rotation "0.000000,180.000000,0.000000")))
      (if (== (Utilities|Array|Length (Collision|GetOverlappingActors (Variables|Default|GetHitbox) 0 :!class /Script/Engine.PrimitiveComponent)) 0)
        _
        (else
          (return false)))))
  (return true))

(fn SetTransform
  (params (SC%20Spawn%20At :type Scene%20Component%20Object%20Reference) (SC%20Origin :type Scene%20Component%20Object%20Reference) (Inverted :type Boolean))
  (bind _returnvalue (Transformation|GetWorldTransform SC%20Spawn%20At))
  (bind _returnvalue_2 (Transformation|GetRelativeTransform SC%20Origin))
  (bind _returnvalue_3 (Math|Transform|InvertTransform _returnvalue_2))
  (bind (_location _rotation) (Math|Transform|BreakTransform _returnvalue))
  (bind _returnvalue_4 (Math|Transform|SelectTransform _returnvalue_3 _returnvalue_2 Inverted))
  (bind (_location_2 _rotation_2) (Math|Transform|BreakTransform _returnvalue_4))
  (Transformation|SetActorTransform (Math|Transform|MakeTransform (Utilities|Operators|Subtract _location _location_2 "0.000000,0.000000,-100.000000") (Math|Rotator|CombineRotators _rotation _rotation_2)))
  (return))

(fn SetorResetOrigin
  (params (Origin%20To :type Scene%20Component%20Object%20Reference) (Reset :type Boolean))
  (bind _root (Variables|Default|GetROOT))
  (Transformation|ResetRelativeTransform _root) ; Reset Transform if a connector changed the origin previously
  (if (not Reset)
    (Transformation|SetRelativeTransform _root (Math|Transform|InvertTransform (Transformation|GetRelativeTransform Origin%20To)) false true)))

(fn GetOverlappingActors
  (bind _overlapping (LocalVariables|GetOverlapping))
  (for _array_element (Components|GetChildrenComponents (Variables|Default|GetPositionalValidators) true)
    (bind _asprimitive_component (Utilities|Casting|CastToPrimitiveComponent _array_element))
    (for _array_element_2 (Collision|GetOverlappingActors _asprimitive_component "BP_HallTemplate_C" :!class /Script/Engine.PrimitiveComponent)
      (if (not (== _array_element_2 self))
        (Utilities|Array|AddUnique (LocalVariables|GetOverlapping) _array_element_2))))
  (return (> (Utilities|Array|Length _overlapping) 0) _overlapping))

(fn GetOUTConnector
  (return (Variables|Default|GetOutConnector)))

(fn RemoveComponents
  (params (Is%20Out%20Components :type Boolean))
  (for _index (range 0 1)
    (for _array_element (Components|GetChildrenComponents (select Is%20Out%20Components (Variables|Default|GetOutComponents) (Variables|Default|GetInComponents)) true)
      (Utilities|IsValid _array_element
        (:Is%20Valid
          (Components|DestroyComponent _array_element))))))