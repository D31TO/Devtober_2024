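; BP_ShellManager spawns AmmoPickup actors as shells at random spots from a supplied location list.
; SpawnShells loops up to the smaller of NumShells and the location count, removing a random entry after each spawn, drawn separately from the spawn pick.
; A WeightedRandom helper, not called here, totals map weights and subtracts them until reaching a random threshold, so higher weights are more common.
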(event Custom|Spawn%20Shells
  (params (Spawn%20Locations :type Array%20of%20Scene%20Component%20Object%20References) (Num%20Shells :type Integer))
  (bind (_outitem _outindex) (Utilities|Array|Random Spawn%20Locations))
  (for _index (range 0 (Math|Integer|Min(Integer) Num%20Shells (Utilities|Array|Length Spawn%20Locations)))
    (Game|SpawnActorfromClass "/Game/Assets/AmmoPickup.AmmoPickup_C" (Transformation|GetWorldTransform _outitem) "Undefined" "MultiplyWithRoot" 0 0)
    (Utilities|Array|RemoveIndex Spawn%20Locations _outindex)))

(fn ConstructionScript)

(fn WeightedRandom
  (params (Selection :type Map%20of%20BP%20Enemy%20Template%20Class%20References%20to%20Reals))
  ;[0.3025 0.4105 0.7083] Random selection from weights (higher is more common)
  (bind _keys (Utilities|Map|Keys Selection))
  (for _array_element _keys
    (bind _output_get (Variables|Default|SetCounter (+ (stale _output_get) (.Value (Utilities|Map|Find Selection _array_element))))))
  (Variables|Default|SetChosen (Math|Random|RandomFloatinRange 0.0 (Variables|Default|GetCounter)))
  (bind _keys_2 (Utilities|Map|Keys Selection))
  (for _array_element_2 _keys_2
    (bind _output_get_2 (Variables|Default|SetCounter (- (Variables|Default|GetCounter) (.Value (Utilities|Map|Find Selection _array_element_2)))))
    (if (<= _output_get_2 (Variables|Default|GetChosen))
      (return _array_element_2))))