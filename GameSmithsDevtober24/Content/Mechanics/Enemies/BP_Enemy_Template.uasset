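; Template enemy character that deals damage, takes damage and awards a coin to the game instance when it dies.
; Hits send damage through BPI_Damage_Handling and trigger OnHitting on the enemy anim Blueprint, while incoming damage lowers Health until the actor is destroyed.
; RandomRoam chains AI moves to random reachable points, MovementSpeed sets walk speed, and BeginPlay and the old Attack event are empty.
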(event Custom|RandomRoam
  ;[1 1 1] Random roam
  (AI|AIMoveTo self (.RandomLocation (AI|Navigation|GetRandomReachablePointinRadius (Transformation|GetActorLocation) 2.5e+03 0 0)) 0 5.0 false
    (:OnSuccess
      (CallFunction|RandomRoam))))

(event Custom|Attack
  (params (PlayerActor :type Actor%20Object%20Reference))
  ;[1 0.5325 0] OLD CODE (MIGHT NEED)
)

(event Custom|Hitting%20the%20player
  (params (Enemy :type Actor%20Object%20Reference))
  ;[0.7292 0 0.06011] Damage
  (if (Utilities|DoesObjectImplementInterface Enemy "/Game/Interfaces/BPI_Damage_Handling.BPI_Damage_Handling_C")
    (Class|BPIDamageHandling|TakeDamage(Message) Enemy (Variables|Default|GetDamage))
    (bind _asabp_enemy_animation (Utilities|Casting|CastToABP_EnemyAnimation (Components|SkeletalMesh|GetAnimInstance (Variables|Character|GetMesh))))
    (Default|OnHitting _asabp_enemy_animation)))

(event EventTakeDamage
  (params (Amount :type Float%20%28double-precision%29))
  ;[0 1 0.1067] Health
  (Variables|Default|SetHealth (- (Variables|Default|GetHealth) Amount))
  (if (<= (Variables|Default|GetHealth) 0.0)
    (Actor|DestroyActor)
    ;[1 0.9317 0] Getting Coins
    (bind _asprim_game_instance (Utilities|Casting|CastToPrimGameInstance (Game|GetGameInstance)))
    (Variables|/Game/GameInstances/PrimGameInstance.PrimGameInstance_C|SetPCoins _asprim_game_instance (+ (Variables|/Game/GameInstances/PrimGameInstance.PrimGameInstance_C|GetPCoins _asprim_game_instance) 1))
    (else
      (Development|PrintString (Utilities|String|ToString(Float) (Variables|Default|GetHealth))))))

(event EventBeginPlay)

(fn ConstructionScript)

(fn MovementSpeed
  (params (NewWalkSpeed :type Float%20%28double-precision%29))
  (Variables|/Script/Engine.CharacterMovementComponent|SetMaxWalkSpeed (Variables|Character|GetCharacterMovement) NewWalkSpeed))