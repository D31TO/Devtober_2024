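; BP_ReboundPad is a scalable box pad that bounces the first-person character off whichever face it hits.
; The construction script scales the pad from BoxScale and fits six thin trigger boxes just outside its faces.
; An overlap passes its face to ReboundActor, which checks cooldown and minimum speed.
; It then mirrors velocity about that face's normal, preserving speed, and launches the character through BPI_PlayerCharacter.
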(event OnComponentBeginOverlap(RightCollision)
  (params (OverlappedComponent :type Primitive%20Component%20Object%20Reference) (OtherActor :type Actor%20Object%20Reference) (OtherComp :type Primitive%20Component%20Object%20Reference) (OtherBodyIndex :type Integer) (bFromSweep :type Boolean) (SweepResult :type Hit%20Result%20Structure%20%28by%20ref%29))
  (if (== (Utilities|GetClass OtherActor) "/Game/FirstPerson/Blueprints/BP_FirstPersonCharacter.BP_FirstPersonCharacter_C")
    (CallFunction|ReboundActor OtherActor "NewEnumerator3")))

(event OnComponentBeginOverlap(LeftCollision)
  (params (OverlappedComponent :type Primitive%20Component%20Object%20Reference) (OtherActor :type Actor%20Object%20Reference) (OtherComp :type Primitive%20Component%20Object%20Reference) (OtherBodyIndex :type Integer) (bFromSweep :type Boolean) (SweepResult :type Hit%20Result%20Structure%20%28by%20ref%29))
  (if (== (Utilities|GetClass OtherActor) "/Game/FirstPerson/Blueprints/BP_FirstPersonCharacter.BP_FirstPersonCharacter_C")
    (CallFunction|ReboundActor OtherActor "NewEnumerator2")))

(event OnComponentBeginOverlap(FrontCollision)
  (params (OverlappedComponent :type Primitive%20Component%20Object%20Reference) (OtherActor :type Actor%20Object%20Reference) (OtherComp :type Primitive%20Component%20Object%20Reference) (OtherBodyIndex :type Integer) (bFromSweep :type Boolean) (SweepResult :type Hit%20Result%20Structure%20%28by%20ref%29))
  (if (== (Utilities|GetClass OtherActor) "/Game/FirstPerson/Blueprints/BP_FirstPersonCharacter.BP_FirstPersonCharacter_C")
    (CallFunction|ReboundActor OtherActor "NewEnumerator0")))

(event OnComponentBeginOverlap(BackCollision)
  (params (OverlappedComponent :type Primitive%20Component%20Object%20Reference) (OtherActor :type Actor%20Object%20Reference) (OtherComp :type Primitive%20Component%20Object%20Reference) (OtherBodyIndex :type Integer) (bFromSweep :type Boolean) (SweepResult :type Hit%20Result%20Structure%20%28by%20ref%29))
  (if (== (Utilities|GetClass OtherActor) "/Game/FirstPerson/Blueprints/BP_FirstPersonCharacter.BP_FirstPersonCharacter_C")
    (CallFunction|ReboundActor OtherActor "NewEnumerator1")))

(event OnComponentBeginOverlap(TopCollision)
  (params (OverlappedComponent :type Primitive%20Component%20Object%20Reference) (OtherActor :type Actor%20Object%20Reference) (OtherComp :type Primitive%20Component%20Object%20Reference) (OtherBodyIndex :type Integer) (bFromSweep :type Boolean) (SweepResult :type Hit%20Result%20Structure%20%28by%20ref%29))
  (if (== (Utilities|GetClass OtherActor) "/Game/FirstPerson/Blueprints/BP_FirstPersonCharacter.BP_FirstPersonCharacter_C")
    (CallFunction|ReboundActor OtherActor "NewEnumerator4")))

(event OnComponentBeginOverlap(BottomCollision)
  (params (OverlappedComponent :type Primitive%20Component%20Object%20Reference) (OtherActor :type Actor%20Object%20Reference) (OtherComp :type Primitive%20Component%20Object%20Reference) (OtherBodyIndex :type Integer) (bFromSweep :type Boolean) (SweepResult :type Hit%20Result%20Structure%20%28by%20ref%29))
  (if (== (Utilities|GetClass OtherActor) "/Game/FirstPerson/Blueprints/BP_FirstPersonCharacter.BP_FirstPersonCharacter_C")
    (CallFunction|ReboundActor OtherActor "NewEnumerator5")))

(fn ConstructionScript
  (bind _boxscale (Variables|Default|GetBoxScale))
  (Transformation|SetWorldScale3D (Variables|Default|GetPad) _boxscale)
  (CallFunction|SetHitboxTransform _boxscale "1.000000,0.000000,0.000000" (Variables|Default|GetLeftCollision) false)
  (CallFunction|SetHitboxTransform _boxscale "1.000000,0.000000,0.000000" (Variables|Default|GetRightCollision) true)
  (CallFunction|SetHitboxTransform _boxscale "0.000000,1.000000,0.000000" (Variables|Default|GetFrontCollision) false)
  (CallFunction|SetHitboxTransform _boxscale "0.000000,1.000000,0.000000" (Variables|Default|GetBackCollision) true)
  (CallFunction|SetHitboxTransform _boxscale "0.000000,0.000000,1.000000" (Variables|Default|GetTopCollision) false)
  (CallFunction|SetHitboxTransform _boxscale "0.000000,0.000000,1.000000" (Variables|Default|GetBottomCollision) true))

(fn ReboundActor
  (params (Target%20Actor :type Actor%20Object%20Reference) (Impact%20Face :type S_NormalFace%20Enum :default "NewEnumerator0"))
  (bind _returnvalue (Transformation|GetVelocity Target%20Actor))
  (bind _returnvalue_2 (Transformation|GetActorForwardVector))
  (bind _returnvalue_3 (Transformation|GetActorUpVector))
  (bind _returnvalue_4 (Transformation|GetActorRightVector))
  (bind _returnvalue_5 (Utilities|Time|GetGameTimeinSeconds))
  (bind _returnvalue_6 (Math|Vector|VectorLength _returnvalue))
  ;[1 0.3842 0.2864] Are we on cooldown?
  (if (>= _returnvalue_5 (+ (Variables|Default|GetCooldownStartTime) (Variables|Default|GetCooldownDuration)))
    ;[0.8895 1 0.4268] Are we moving fast enough to rebound?
    (if (>= _returnvalue_6 (Variables|Default|GetMinimumInitialVelocity))
      (Development|PrintString (Utilities|String|Append "Initial Velocity: " (Utilities|String|ToString(Float) _returnvalue_6)))
      (Variables|Default|SetCooldownStartTime _returnvalue_5)
      (if (Utilities|DoesObjectImplementInterface Target%20Actor "/Game/Interfaces/BPI_PlayerCharacter.BPI_PlayerCharacter_C")
        (Class|BPIPlayerCharacter|ApplyLaunchVelocity(Message) Target%20Actor (* (Math|Vector|VectorLength _returnvalue) (Math|Vector|MirrorVectorbyNormal (Math|Vector|Normalize _returnvalue) (* (Utilities|Select :Index Impact%20Face :NewEnumerator0 (* _returnvalue_4 -1) :NewEnumerator1 _returnvalue_4 :NewEnumerator2 (* _returnvalue_2 -1) :NewEnumerator3 _returnvalue_2 :NewEnumerator4 _returnvalue_3 :NewEnumerator5 (* _returnvalue_3 -1)) 1)) 1) true)))))

(fn SetHitboxTransform
  (params (Scale :type Vector) (TargetAxis :type Vector) (Hitbox%20Target :type Box%20Component%20Object%20Reference) (IsInverted :type Boolean))
  (bind _hitboxsizetounitscalefactor (Variables|Default|GetHitboxSizeToUnitScaleFactor))
  (bind _hitboxdepthsize (Variables|Default|GetHitboxDepthSize))
  (bind _returnvalue (* _hitboxsizetounitscalefactor Scale))
  (if (== (.x TargetAxis) 1.0) ; if X is 1, must be L/R
    (Components|Box|SetBoxExtent Hitbox%20Target (Math|Vector|MakeVector _hitboxdepthsize (.y _returnvalue) (.z _returnvalue)) true)
    (Transformation|SetRelativeLocation Hitbox%20Target (Math|Vector|MakeVector (CallFunction|GetHitboxOffsetLocation (.x _returnvalue) IsInverted) 0.0 0.0) false false)
    (elif (== (.y TargetAxis) 1.0) ; if Y is 1, must be U/D
      (Components|Box|SetBoxExtent Hitbox%20Target (Math|Vector|MakeVector (.x _returnvalue) _hitboxdepthsize (.z _returnvalue)) true)
      (Transformation|SetRelativeLocation Hitbox%20Target (Math|Vector|MakeVector 0.0 (CallFunction|GetHitboxOffsetLocation (.y _returnvalue) IsInverted) 0.0) false false)
      (elif (== (.z TargetAxis) 1.0) ; if Z is 1, must be F/B
        (Components|Box|SetBoxExtent Hitbox%20Target (Math|Vector|MakeVector (.x _returnvalue) (.y _returnvalue) _hitboxdepthsize) true)
        (Transformation|SetRelativeLocation Hitbox%20Target (Math|Vector|MakeVector 0.0 0.0 (CallFunction|GetHitboxOffsetLocation (.z _returnvalue) IsInverted)) false false)))))

(fn GetHitboxOffsetLocation
  (params (Scale%20%28In%20Extent%29 :type Float%20%28double-precision%29) (Inverted :type Boolean))
  (return (* (+ Scale%20%28In%20Extent%29 (Variables|Default|GetHitboxDepthSize)) (Math|Integer|SelectInt -1 1 Inverted))))